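; Food component that makes an interactable pickup edible on the spot or storable in the player's inventory.
; On BeginPlay it binds eating to the Use event and storing to the Interact event of BpInter.
; Eating adds ObtainHunger to PlayerControllerMetus's Hunger, while storing sets HasFood and FoodType only if no food is already held.
; Either successful action disables input on the BpInter actor and destroys it.
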(event `self.ReceiveBeginPlay`
  (bind _bpinter (`self.bpInter`))
  (add `/Game/Custom/Blueprints/BP_Interactible.Event_Use` _bpinter (delegate `Eat_in_place`))
  (add `/Game/Custom/Blueprints/BP_Interactible.Event_Interact` _bpinter (delegate `Put_in_inventory`))
  (`KismetSystemLibrary.PrintString` "event use bind"))

(event `Eat_in_place`
  (bind _returnvalue (`GameplayStatics.GetPlayerController` 0))
  (bind _bpinter (`self.bpInter`))
  (bind _asplayer_controller_metus (cast `/Game/Custom/Blueprints/Character/PlayerControllerMetus` _returnvalue))
  (set `/Game/Custom/Blueprints/Character/PlayerControllerMetus.Hunger` (+ (`/Game/Custom/Blueprints/Character/PlayerControllerMetus.Hunger` _asplayer_controller_metus) (`self.Obtain_Hunger`)) _asplayer_controller_metus)
  (`Actor.DisableInput` _bpinter _returnvalue :!label _label)
  (`Actor.K2_DestroyActor` _bpinter))

(event `Put_in_inventory`
  (bind _asplayer_controller_metus (cast `/Game/Custom/Blueprints/Character/PlayerControllerMetus` (`GameplayStatics.GetPlayerController` 0)))
  (if (not (`/Game/Custom/Blueprints/Character/PlayerControllerMetus.Has_food` _asplayer_controller_metus))
    (set `/Game/Custom/Blueprints/Character/PlayerControllerMetus.Has_food` true _asplayer_controller_metus)
    (set `/Game/Custom/Blueprints/Character/PlayerControllerMetus.Food_type` (`self.Food`) _asplayer_controller_metus)
    (goto _label)))
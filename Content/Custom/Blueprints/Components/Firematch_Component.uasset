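; Actor component that turns an interactable into a collectible firematch for the player.
; On BeginPlay it binds to the interact event of its BpInteract reference.
; On interaction, if the PlayerControllerMetus firematch count is below MaxFirematches, it sets HasFirematch, increments the count, disables input on the interact actor and destroys it.
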(event `self.ReceiveBeginPlay`
  (add `/Game/Custom/Blueprints/BP_Interactible.Event_Interact` (`self.BpInteract`) (delegate `Put_in_inventory`)))

(event `Put_in_inventory`
  (bind _returnvalue (`GameplayStatics.GetPlayerController` 0))
  (bind _bpinteract (`self.BpInteract`))
  (bind _asplayer_controller_metus (cast `/Game/Custom/Blueprints/Character/PlayerControllerMetus` _returnvalue))
  (if (< (`/Game/Custom/Blueprints/Character/PlayerControllerMetus.Firematch_num` _asplayer_controller_metus) (`self.Max_firematches`))
    (set `/Game/Custom/Blueprints/Character/PlayerControllerMetus.Has_Firematch` true _asplayer_controller_metus)
    (set `/Game/Custom/Blueprints/Character/PlayerControllerMetus.Firematch_num` (+ (`/Game/Custom/Blueprints/Character/PlayerControllerMetus.Firematch_num` _asplayer_controller_metus) 1) _asplayer_controller_metus)
    (`Actor.DisableInput` _bpinteract _returnvalue)
    (`Actor.K2_DestroyActor` _bpinteract)))
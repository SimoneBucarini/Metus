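; Pickup actor for food, medicine or firematches, with its mesh set from the chosen type at construction.
; A box overlap enables input and type-specific prompts: Interact adds the item to the Cooldown game instance, while Use in place raises Hunger or Health.
; Pickups and used medicine move below the map until Spawn restores them.
; Eaten food stays put, and its random poison roll leaves Health unchanged.
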(event `InputAction|Use in place`
  (params (Key :type "Key Structure"))
  (bind _ascooldown (cast `/Game/Custom/Blueprints/Cores/Cooldown` (`GameplayStatics.GetGameInstance`) :!pure true))
  ;[1 1 1] Y interaction
  (:`Pressed`
    (if (`self.In_Range`)
      (switch `/Game/Custom/Blueprints/ENUM_interactible_old` (cast `/Game/Custom/Blueprints/ENUM_interactible_old` (`self.Type Choise`))
        (:`NewEnumerator1`
          (bind _output_get (set `self.Poisoned` (> (`KismetMathLibrary.RandomInteger` 100) 95)))
          (if _output_get
            (set `/Game/Custom/Blueprints/Cores/Cooldown.Health` (`/Game/Custom/Blueprints/Cores/Cooldown.Health` _ascooldown) _ascooldown))
          (set `/Game/Custom/Blueprints/Cores/Cooldown.Hunger` (+ (`/Game/Custom/Blueprints/Cores/Cooldown.Hunger` _ascooldown) 0.2) _ascooldown))
        (:`NewEnumerator2`
          (set `/Game/Custom/Blueprints/Cores/Cooldown.Health` (+ (`/Game/Custom/Blueprints/Cores/Cooldown.Health` _ascooldown) 0.2) _ascooldown)
          (`self.K2_SetActorLocation` (0.0 0.0 -1000.0) :!label _label)
          (set `self.Exists` false))))))

(event `InputAction|Interact`
  (params (Key :type "Key Structure"))
  (bind _ascooldown (cast `/Game/Custom/Blueprints/Cores/Cooldown` (`GameplayStatics.GetGameInstance`) :!pure true))
  (:`Pressed`
    (if (`self.In_Range`)
      (switch `/Game/Custom/Blueprints/ENUM_interactible_old` (cast `/Game/Custom/Blueprints/ENUM_interactible_old` (`self.Type Choise`))
        (:`NewEnumerator0`
          ;[1 1 1] +Firematch
          (`/Game/Custom/Blueprints/Cores/Cooldown.Add_Firematch` _ascooldown)
          (`self.UI_Update`)
          (goto _label))
        (:`NewEnumerator1`
          ;[1 1 1] + Food
          (`/Game/Custom/Blueprints/Cores/Cooldown.Add_Food` _ascooldown)
          (`self.UI_Update`)
          (goto _label))
        (:`NewEnumerator2`
          ;[1 1 1] + Medicine
          (`/Game/Custom/Blueprints/Cores/Cooldown.Add_Medicines` _ascooldown)
          (`self.UI_Update`)
          (goto _label))))))

(event `self.Box.OnComponentBeginOverlap`
  (params (OverlappedComponent :type "PrimitiveComponent Object Reference") (OtherActor :type "Actor Object Reference") (OtherComp :type "PrimitiveComponent Object Reference") (OtherBodyIndex :type Integer) (bFromSweep :type Boolean) (SweepResult :type "HitResult Structure (by ref)"))
  ;[1 1 1] UI Prompt Spawn
  (set `self.In_Range` true)
  (`self.EnableInput` (`GameplayStatics.GetPlayerController` 0))
  (bind _returnvalue (`|CreateWidget` "/Game/Custom/Widget/X_Pickup.X_Pickup_C"))
  (`UserWidget.AddToViewport` _returnvalue 0)
  (switch `/Game/Custom/Blueprints/ENUM_interactible_old` (cast `/Game/Custom/Blueprints/ENUM_interactible_old` (`self.Type Choise`))
    (:`NewEnumerator1`
      (bind _returnvalue_2 (`|CreateWidget` "/Game/Custom/Widget/Y_Eat.Y_Eat_C"))
      (`UserWidget.AddToViewport` _returnvalue_2 0))
    (:`NewEnumerator2`
      (bind _returnvalue_3 (`|CreateWidget` "/Game/Custom/Widget/Y_UseMedicine.Y_UseMedicine_C"))
      (`UserWidget.AddToViewport` _returnvalue_3 0))))

(event `self.Box.OnComponentEndOverlap`
  (params (OverlappedComponent :type "PrimitiveComponent Object Reference") (OtherActor :type "Actor Object Reference") (OtherComp :type "PrimitiveComponent Object Reference") (OtherBodyIndex :type Integer))
  ;[1 1 1] UI Prompt Spawn
  (set `self.In_Range` false)
  (`self.DisableInput` (`GameplayStatics.GetPlayerController` 0))
  (`Widget.RemoveFromParent` (stale `self.Box.OnComponentBeginOverlap` _returnvalue))
  (switch `/Game/Custom/Blueprints/ENUM_interactible_old` (cast `/Game/Custom/Blueprints/ENUM_interactible_old` (`self.Type Choise`))
    (:`NewEnumerator1`
      (`Widget.RemoveFromParent` (stale `self.Box.OnComponentBeginOverlap` _returnvalue_2)))
    (:`NewEnumerator2`
      (`Widget.RemoveFromParent` (stale `self.Box.OnComponentBeginOverlap` _returnvalue_3)))))

(event `Spawn`
  (`self.K2_SetActorLocation` (`self.Location`))
  (set `self.Exists` true))

(event `UI_Update`
  (bind _ascooldown (cast `/Game/Custom/Blueprints/Cores/Cooldown` (`GameplayStatics.GetGameInstance`) :!pure true))
  (bind _ui (`/Game/Custom/Blueprints/Cores/Cooldown.UI` _ascooldown))
  (`EditableTextBox.SetHintText` (`/Game/Custom/Widget/UI_StatusBars.Firematch` _ui) (`KismetTextLibrary.Conv_IntToText` (`/Game/Custom/Blueprints/Cores/Cooldown.Firematch` _ascooldown)))
  (`EditableTextBox.SetHintText` (`/Game/Custom/Widget/UI_StatusBars.Food` _ui) (`KismetTextLibrary.Conv_IntToText` (`/Game/Custom/Blueprints/Cores/Cooldown.Food` _ascooldown)))
  (`EditableTextBox.SetHintText` (`/Game/Custom/Widget/UI_StatusBars.Medicine` _ui) (`KismetTextLibrary.Conv_IntToText` (`/Game/Custom/Blueprints/Cores/Cooldown.Medicines` _ascooldown))))

(fn `UserConstructionScript`
  (locals (`Mesh Array` :type "Array of StaticMesh Object Reference"))
  (`StaticMeshComponent.SetStaticMesh` (`self.StaticMesh`) (`|GetArrayItem` (`local.Mesh Array`) (`KismetMathLibrary.Conv_ByteToInt` (`self.Type Choise`)))))
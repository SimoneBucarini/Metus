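; Player controller for a survival game, holding health, hunger, sleep, sanity, stamina, item counts and a day clock.
; Looping named timers advance time and drain needs, with sanity falling outside light.
; Item functions handle limits, poisoned food and timed warning widgets, while resting fades the camera, skips a day and restores sleep.
; HUD creation, parameter setup and the health-decay body are disconnected, though functions still update the old UI reference.
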(event `InputAction|Use Medicine`
  (params (Key :type "Key Structure"))
  (:`Pressed`
    (`self.Add_Medicines`)))

(event `InputAction|Use Food`
  (params (Key :type "Key Structure"))
  (:`Pressed`
    (`self.Use_Food`)))

(event `Death`
  (bind _returnvalue (`GameplayStatics.GetPlayerController` 0))
  (`self.DisableInput` (`GameplayStatics.GetPlayerPawn` 0) _returnvalue)
  (bind _returnvalue_2 (`|CreateWidget` "/Game/Custom/Widget/DeathScreen.DeathScreen_C" _returnvalue))
  (`UserWidget.AddToViewport` _returnvalue_2 0)
  (set `PlayerController.bShowMouseCursor` true _returnvalue))

(event `self.ReceiveBeginPlay`
  (`|ExecutionSequence`
    (:`then_1`
      (`KismetSystemLibrary.K2_SetTimer` null "Time" (`self.System Clock`) true)
      (`KismetSystemLibrary.K2_SetTimer` null "Sanity_timer" (`self.Sanity_timer_frequency`) true)
      (`KismetSystemLibrary.K2_SetTimer` null "Hunger_timer" (`self.Hunger_timer_frequency`) true)
      (`KismetSystemLibrary.K2_SetTimer` null "Sleep_Timer" (`self.Sleep__timer_frequency`) true)
      (`KismetSystemLibrary.K2_SetTimer` null "Health_degrowth_by_sanity_and_hunger" (`self.Health_timer_frequency`) true))))

(event `Too_Much_Medicines`
  (if (not (`self.Cooldown`))
    (bind _returnvalue (`|CreateWidget` "/Game/Custom/Widget/Too_Much_Medikits.Too_Much_Medikits_C"))
    (`UserWidget.AddToViewport` _returnvalue 0)
    (set `self.Cooldown` true)
    (`KismetSystemLibrary.Delay` 1.2)
    (set `self.Cooldown` false)
    (`Widget.RemoveFromParent` _returnvalue)))

(event `Too_Much_Food`
  (if (not (`self.Cooldown`))
    (bind _returnvalue (`|CreateWidget` "/Game/Custom/Widget/Too_Much_Food.Too_Much_Food_C"))
    (`UserWidget.AddToViewport` _returnvalue 0)
    (set `self.Cooldown` true)
    (`KismetSystemLibrary.Delay` 1.2)
    (set `self.Cooldown` false)
    (`Widget.RemoveFromParent` _returnvalue)))

(event `Use_Food1`
  (if (<= (`self.Food`) 0)
    (if (not (`self.Cooldown`))
      (bind _returnvalue (`|CreateWidget` "/Game/Custom/Widget/Dont_Have_Food.Dont_Have_Food_C"))
      (`UserWidget.AddToViewport` _returnvalue 0)
      (set `self.Cooldown` true)
      (`KismetSystemLibrary.Delay` 2.0)
      (set `self.Cooldown` false)
      (`Widget.RemoveFromParent` _returnvalue))
    (else
      (`self.Use_Food`)
      (if (`self.Poisoned_Character`)
        (set `self.Poisoned_Character` false)
        (bind _returnvalue_2 (`|CreateWidget` "/Game/Custom/Widget/Poisoned_Food.Poisoned_Food_C"))
        (`UserWidget.AddToViewport` _returnvalue_2 0)
        (`KismetSystemLibrary.Delay` 2.0)
        (`Widget.RemoveFromParent` _returnvalue_2)))))

(event `Decrease Stamina`
  (bind _output_get (set `self.Stamina` (- (`self.Stamina`) (`self.Sprint_decrementation`))))
  (set `self.Stop_stamina_drain` (<= _output_get 0.0)))

(event `Stamina Incrementation`
  (bind _output_get (set `self.Stamina` (+ (`self.Stamina`) (`self.Sprint_incrementation`))))
  (set `self.Stop_stamina_regen` (>= _output_get 1.0)))

(event `Use_Medicine1`
  (if (<= (`self.Medicines`) 0)
    (if (not (`self.Cooldown`))
      (bind _returnvalue (`|CreateWidget` "/Game/Custom/Widget/Dont_Have_Medkit.Dont_Have_Medkit_C"))
      (`UserWidget.AddToViewport` _returnvalue 0)
      (set `self.Cooldown` true)
      (`KismetSystemLibrary.Delay` 2.0)
      (set `self.Cooldown` false)
      (`Widget.RemoveFromParent` _returnvalue))
    (else
      (`self.Use_Medicine`))))

(event `Resting`
  (bind _returnvalue (`GameplayStatics.GetPlayerCameraManager` 0))
  (bind _returnvalue_2 (`GameplayStatics.GetPlayerPawn` 0))
  ;[1 1 1] Resting
  (if (`self.is_bed_near?`)
    (`self.DisableInput` _returnvalue_2 (`GameplayStatics.GetPlayerController` 0))
    (`self.Rest`)
    (set `self.Resting?` true)
    (`PlayerCameraManager.StartCameraFade` :`self` _returnvalue :`ToAlpha` 1.0 :`Duration` 2.5 :`bHoldWhenFinished` true)
    (`KismetSystemLibrary.Delay` 2.5)
    (`PlayerCameraManager.StartCameraFade` :`self` _returnvalue :`FromAlpha` 1.0 :`Duration` 2.5 :`bHoldWhenFinished` true)
    (`KismetSystemLibrary.Delay` 2.5)
    (`self.EnableInput` _returnvalue_2 (`GameplayStatics.GetPlayerController` 0))
    (set `self.Resting?` false)))

(fn `Add_Firematch`
  (set `self.Firematch` (+ (`self.Firematch`) 1)))

(fn `Add_Food`
  (bind _returnvalue (+ (`self.Food`) 1))
  (if (>= (`self.Food`) 1)
    (`self.Too_Much_Food`)
    (elif (> (`KismetMathLibrary.RandomInteger` 100) 95)
      (set `self.Food` _returnvalue)
      (set `self.Poisoned_Character` true)
      (else
        (set `self.Food` _returnvalue)))))

(fn `Add_Medicines`
  (bind _medicines (`self.Medicines`))
  (if (>= _medicines 1)
    (`self.Too_Much_Medicines`)
    (else
      (set `self.Medicines` (+ _medicines 1)))))

(fn `Create_UI`
  ;[1 1 1] Create UI
  (bind _returnvalue (`|CreateWidget` "/Game/Custom/Widget/UI_StatusBars.UI_StatusBars_C"))
  (bind _output_get (set `self.UI_OLD` _returnvalue))
  (`UserWidget.AddToViewport` _output_get 0))

(fn `Health_degrowth_by_sanity_and_hunger`)

(fn `Hunger_timer`
  (bind _returnvalue (- (`self.Hunger`) (`self.Hunger_decrementation`)))
  (bind _returnvalue_2 (<= _returnvalue 0.0))
  (if _returnvalue_2
    (set `self.Is_hunger_zero?` _returnvalue_2 :!label _label)
    (set `self.Hunger` 0.0)
    (else
      (set `self.Is_hunger_zero?` _returnvalue_2)
      (if (`self.Is_hunger_zero?`)
        (goto _label)
        (else
          (set `self.Hunger` _returnvalue))))))

(fn `Init_Parameters`)

(fn `Rest`
  (bind _sleep (`self.Sleep`))
  (bind _ui_old (`self.UI_OLD`))
  (bind _returnvalue (+ (`self.Days`) 1))
  (set `self.Seconds` 0)
  (bind _output_get (set `self.Hours` 8))
  (set `self.Days` _returnvalue)
  (`EditableTextBox.SetHintText` (`/Game/Custom/Widget/UI_StatusBars.Hours` _ui_old) (`KismetTextLibrary.Conv_ByteToText` _output_get))
  (`EditableTextBox.SetHintText` (`/Game/Custom/Widget/UI_StatusBars.Days` _ui_old) (`KismetTextLibrary.Conv_IntToText` _returnvalue))
  (if (< _sleep 0.3)
    (set `self.Sleep` 0.75)
    (else
      (set `self.Sleep` 1.0)))
  (`ProgressBar.SetPercent` (`/Game/Custom/Widget/UI_StatusBars.SleepBar` _ui_old) _sleep))

(fn `Sanity_timer`
  (bind _sanity (`self.Sanity`))
  (bind _returnvalue (- _sanity (`self.Sanity_decrementation`)))
  (bind _returnvalue_2 (<= _returnvalue 1e-05))
  (if (`self.Resting?`)
    _
    (elif (not (`self.Is_in_light?`))
      (if (>= _sanity 1.0)
        (set `self.Sanity` 1.0))
      (if _returnvalue_2
        (set `self.Is_sanity_zero?` _returnvalue_2 :!label _label)
        (elif (`self.Is_sanity_zero?`)
          (goto _label)
          (else
            (bind _output_get (set `self.Sanity` _returnvalue))
            (if (> _output_get 0.75)
              ;[1 1 1] Sanity Rannge Flags Settings
              (set `self.Low_Saniry` false)
              (set `self.Medium_Sanity` false)
              (set `self.Full_Sanity` true)
              (elif (> _output_get 0.3)
                (set `self.Low_Saniry` false)
                (set `self.Medium_Sanity` true)
                (set `self.Full_Sanity` false)
                (else
                  (set `self.Low_Saniry` true)
                  (set `self.Medium_Sanity` false)
                  (set `self.Full_Sanity` false))))))))))

(fn `Sleep_Timer`
  (bind _returnvalue (- (`self.Sleep`) (`self.Sleep_Decrementation`)))
  (bind _returnvalue_2 (<= _returnvalue 0.0))
  (if _returnvalue_2
    (set `self.Is_sleep_zero?` _returnvalue_2 :!label _label)
    (set `self.Sleep` 0.0)
    (else
      (set `self.Is_sleep_zero?` _returnvalue_2)
      (if (`self.Is_sleep_zero?`)
        (goto _label)
        (else
          (set `self.Sleep` _returnvalue))))))

(fn `Sprint_dec_by_freq`
  (if (`self.Stop_stamina_drain`)
    (set `self.Stamina` (- (`self.Stamina`) (`self.Sprint_decrementation`)))
    (else
      (set `self.Stamina` (+ (`self.Stamina`) (`self.Sprint_incrementation`))))))

(fn `Time`
  (bind _output_get (set `self.Seconds` (+ (`self.Seconds`) 1)))
  (if (>= _output_get 1)
    (set `self.Seconds` 0)
    (bind _output_get_2 (set `self.Minutes` (+ (`self.Minutes`) 1)))
    (if (>= _output_get_2 60)
      (set `self.Minutes` 0)
      (bind _output_get_3 (set `self.Hours` (+ (`self.Hours`) 1)))
      (if (>= _output_get_3 24)
        (set `self.Hours` 0)
        (set `self.Days` (+ (`self.Days`) 1))
        (`/Engine/EditorBlueprintResources/StandardMacros.DoOnce` false :!via `Reset`)))))

(fn `Use_Food`
  (bind _food (`self.Food`))
  (bind _ui_old (`self.UI_OLD`))
  (bind _ui_old_2 (`self.UI_OLD`))
  (bind _food_2 (`self.Food`))
  (if (`self.Poisoned_Character`)
    (if (> _food 0)
      (bind _output_get (set `self.Food` (- _food 1)))
      (bind _output_get_2 (set `self.Hunger` (+ (`self.Hunger`) 0.25)))
      (bind _output_get_3 (set `self.Health` (- (`self.Health`) 0.2)))
      (`ProgressBar.SetPercent` (`/Game/Custom/Widget/UI_StatusBars.HealthBar` _ui_old) _output_get_3)
      (`ProgressBar.SetPercent` (`/Game/Custom/Widget/UI_StatusBars.HungerBar` _ui_old) _output_get_2)
      (`EditableTextBox.SetHintText` (`/Game/Custom/Widget/UI_StatusBars.Food` _ui_old) (`KismetTextLibrary.Conv_IntToText` _output_get)))
    (elif (> _food_2 0)
      (bind _output_get_4 (set `self.Food` (- _food_2 1)))
      (bind _output_get_5 (set `self.Hunger` (+ (`self.Hunger`) 0.25)))
      (`ProgressBar.SetPercent` (`/Game/Custom/Widget/UI_StatusBars.HungerBar` _ui_old_2) _output_get_5)
      (`EditableTextBox.SetHintText` (`/Game/Custom/Widget/UI_StatusBars.Food` _ui_old_2) (`KismetTextLibrary.Conv_IntToText` _output_get_4)))))

(fn `Use_Medicine`
  (bind _medicines (`self.Medicines`))
  (bind _ui_old (`self.UI_OLD`))
  (if (> _medicines 0)
    (bind _output_get (set `self.Medicines` (- _medicines 1)))
    (bind _output_get_2 (set `self.Health` (+ (`self.Health`) 0.2)))
    (`ProgressBar.SetPercent` (`/Game/Custom/Widget/UI_StatusBars.HealthBar` _ui_old) _output_get_2)
    (`EditableTextBox.SetHintText` (`/Game/Custom/Widget/UI_StatusBars.Medicine` _ui_old) (`KismetTextLibrary.Conv_IntToText` _output_get))))

(fn `UserConstructionScript`)
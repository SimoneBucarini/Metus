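; BP_Interactible is an interactible actor whose appearance is configured by type in the construction script.
; For the Food type, it uses FoodType as an index into the FoodsData array in InteractibleBulder's FOODDATA, then applies that entry's mesh and material to its StaticMesh.
; Only the Food case has logic, and the event graph contains no runtime behavior.
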(event `self.ReceiveBeginPlay`)

(fn `UserConstructionScript`
  (bind (_hunger_obtained _poison_ratio _mesh _material) (break `/Game/Custom/Blueprints/Stuctures/STRUCT_Food` (`|GetArrayItem` (`.Foods_Data_3_4B6153B246894231944104B87E575E65` (break `/Game/Custom/Blueprints/Stuctures/FOODS_DATA` (`/Game/Custom/Blueprints/Cores/Interaclibles_Builder.FOOD_DATA` (`self.Interactible_bulder`)))) (`KismetMathLibrary.Conv_ByteToInt` (`self.Food_Type`)))))
  (switch `/Game/Custom/Blueprints/Enums/ENUM_interactible` (`self.Interactible_Type`)
    (:`NewEnumerator1`
      (`StaticMeshComponent.SetStaticMesh` (`self.StaticMesh`) _mesh)
      (`PrimitiveComponent.SetMaterial` (`self.StaticMesh`) 0 _material))))
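; Interactibles builder that rebuilds every BP_Interactible actor in the world when Build_Interactibles is called.
; It stores the actor references and count, saves each one's transform, static parameters and randomizer settings into a struct array, then destroys it.
; A second pass spawns a fresh BP_Interactible from each struct and copies the saved parameters back.
; The struct array is appended to without being cleared in this event.
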(event `Build_Interactibles`
  (bind _outactors (`GameplayStatics.GetAllActorsOfClass` "/Game/Custom/Blueprints/BP_Interactible.BP_Interactible_C"))
  (bind _output_get (set `self.Interactibles_References_Array` _outactors))
  (set `self.Iteractible number` (`KismetArrayLibrary.Array_Length` _output_get))
  (for _array_element _output_get
    (bind _output_get_2 (set `self.Struct_Interactible` (make `/Game/Custom/Blueprints/Stuctures/Interactible_STRUCT` (`Actor.GetTransform` _array_element) (`/Game/Custom/Blueprints/BP_Interactible.Static Parameters` _array_element) (`/Game/Custom/Blueprints/BP_Interactible.Randomizer Enable` _array_element) (`/Game/Custom/Blueprints/BP_Interactible.Randomizer Settings` _array_element))))
    (`KismetArrayLibrary.Array_Add` (`self.Array_Struct_Interactible`) _output_get_2)
    (`Actor.K2_DestroyActor` _array_element))
  (for _array_element_2 (`self.Array_Struct_Interactible`)
    (bind (_interactible_transform_parameter _static_interactible_parameters _randomizerenable _randomizer_settings) (break `/Game/Custom/Blueprints/Stuctures/Interactible_STRUCT` _array_element_2))
    (bind _returnvalue (`|SpawnActorFromClass` "/Game/Custom/Blueprints/BP_Interactible.BP_Interactible_C" _interactible_transform_parameter "Undefined" "OverrideRootScale" null null))
    (set `/Game/Custom/Blueprints/BP_Interactible.Static Parameters` _static_interactible_parameters _returnvalue)
    (set `/Game/Custom/Blueprints/BP_Interactible.Randomizer Enable` _randomizerenable _returnvalue)
    (set `/Game/Custom/Blueprints/BP_Interactible.Randomizer Settings` _randomizer_settings _returnvalue)))
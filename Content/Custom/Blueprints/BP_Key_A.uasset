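; BP_Key_A is a pickup actor for Key A that the player collects with the Interact input.
; Overlapping its Box enables input and shows an X_Pickup prompt widget; leaving disables input and removes it.
; Interacting sets KeyA on the Cooldown game instance, destroys the particle and teleports the actor far below the level instead of destroying it, while a Key_A widget shows briefly.
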(event `InputAction|Interact`
  (params (Key :type "Key Structure"))
  (:`Pressed`
    (set `/Game/Custom/Blueprints/Cooldown.Key_A` true (cast `/Game/Custom/Blueprints/Cooldown` (`GameplayStatics.GetGameInstance`) :!pure true))
    (bind _returnvalue (`|CreateWidget` "/Game/Custom/Widget/Key_A.Key_A_C"))
    (`UserWidget.AddToViewport` _returnvalue 0)
    (`ActorComponent.K2_DestroyComponent` (`self.ParticleSystem`))
    (`self.K2_SetActorLocation` (0.0 0.0 -5000.0))
    (`KismetSystemLibrary.Delay` 1.2)
    (`Widget.RemoveFromParent` _returnvalue)))

(event `self.Box.OnComponentBeginOverlap`
  (params (OverlappedComponent :type "PrimitiveComponent Object Reference") (OtherActor :type "Actor Object Reference") (OtherComp :type "PrimitiveComponent Object Reference") (OtherBodyIndex :type Integer) (bFromSweep :type Boolean) (SweepResult :type "HitResult Structure (by ref)"))
  (`self.EnableInput` (`GameplayStatics.GetPlayerController` 0))
  (bind _returnvalue (`|CreateWidget` "/Game/Custom/Widget/X_Pickup.X_Pickup_C"))
  (`UserWidget.AddToViewport` _returnvalue 0))

(event `self.Box.OnComponentEndOverlap`
  (params (OverlappedComponent :type "PrimitiveComponent Object Reference") (OtherActor :type "Actor Object Reference") (OtherComp :type "PrimitiveComponent Object Reference") (OtherBodyIndex :type Integer))
  (`self.DisableInput` (`GameplayStatics.GetPlayerController` 0))
  (`Widget.RemoveFromParent` (stale `self.Box.OnComponentBeginOverlap` _returnvalue)))

(fn `UserConstructionScript`)
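; Torch actor that the player lights with Interact, using up one of the Character's Firematch count.
; A box overlap with the character's capsule arms it and shows a Press_E widget while unlit, and leaving clears both.
; Interact plays a timeline that scales the particle system and point light intensity, sets OnOff and removes the prompt.
; The match is deducted when the timeline finishes, and Interact itself never checks OnOff.
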(event `self.ReceiveBeginPlay`
  (`self.EnableInput` (`GameplayStatics.GetPlayerController` 0)))

(event `self.Box.OnComponentBeginOverlap`
  (params (OverlappedComponent :type "PrimitiveComponent Object Reference") (OtherActor :type "Actor Object Reference") (OtherComp :type "PrimitiveComponent Object Reference") (OtherBodyIndex :type Integer) (bFromSweep :type Boolean) (SweepResult :type "HitResult Structure (by ref)"))
  (if (`self.On/Off`)
    _
    (elif (== (`Character.CapsuleComponent` (`self.Character`)) OtherComp)
      (set `self.Ready` true)
      (bind _returnvalue (`|CreateWidget` "/Game/Custom/Widget/Press_E.Press_E_C"))
      (`UserWidget.AddToViewport` _returnvalue 0))))

(event `InputAction|Interact`
  (params (Key :type "Key Structure"))
  (bind _character (`self.Character`))
  (:`Pressed`
    (if (> (`/Game/Custom/Blueprints/Personaggio.Firematch` (`self.Character`)) 0)
      (if (`self.Ready`)
        (bind (_direction _luce _fuoco) (`Timeline|Timeline_0` :!via `PlayFromStart`)
          (:`Update`
            (`SceneComponent.SetRelativeScale3D` (`self.ParticleSystem`) (`KismetMathLibrary.MakeVector` _fuoco _fuoco _fuoco))
            (`LightComponent.SetIntensity` (`self.PointLight`) (* _luce 5000.0))
            (set `self.On/Off` true)
            (`Widget.RemoveFromParent` (stale `self.Box.OnComponentBeginOverlap` _returnvalue)))
          (:`Finished`
            (set `/Game/Custom/Blueprints/Personaggio.Firematch` (- (`/Game/Custom/Blueprints/Personaggio.Firematch` _character) 1) _character)))))))

(event `self.Box.OnComponentEndOverlap`
  (params (OverlappedComponent :type "PrimitiveComponent Object Reference") (OtherActor :type "Actor Object Reference") (OtherComp :type "PrimitiveComponent Object Reference") (OtherBodyIndex :type Integer))
  (if (== (`Character.CapsuleComponent` (`self.Character`)) OtherComp)
    (set `self.Ready` false)
    (`Widget.RemoveFromParent` (stale `self.Box.OnComponentBeginOverlap` _returnvalue))))

(fn `UserConstructionScript`)
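; Survival stats Blueprint that tracks health, hunger, sanity, sleep, item counts and an in-game clock, mirroring them to a status-bar widget.
; Timer-style functions drain sanity in darkness, plus sleep and hunger; empty sleep or hunger drains health toward a death screen.
; Food, occasionally poisoned, and medicine adjust stats, while resting near a bed fades the camera, advances the day and restores sleep.
; A shared Cooldown flag stops inventory warning popups from stacking.
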(event `Death`
  (bind _returnvalue (`GameplayStatics.GetPlayerController` 0))
  (`Actor.DisableInput` (`GameplayStatics.GetPlayerPawn` 0) _returnvalue)
  (bind _returnvalue_2 (`|CreateWidget` "/Game/Custom/Widget/DeathScreen.DeathScreen_C" _returnvalue))
  (`UserWidget.AddToViewport` _returnvalue_2 0)
  (set `PlayerController.bShowMouseCursor` true _returnvalue))

(event `Too_Much_Medicines`
  (if (not (`self.Cooldown`))
    (bind _returnvalue (`|CreateWidget` "/Game/Custom/Widget/Too_Much_Medikits.Too_Much_Medikits_C"))
    (`UserWidget.AddToViewport` _returnvalue 0)
    (set `self.Cooldown` true)
    (`KismetSystemLibrary.Delay` 1.2)
    (set `self.Cooldown` false)
    (`Widget.RemoveFromParent` _returnvalue)))

(event `Too_Much_Food`
  (if (not (`self.Cooldown`))
    (bind _returnvalue (`|CreateWidget` "/Game/Custom/Widget/Too_Much_Food.Too_Much_Food_C"))
    (`UserWidget.AddToViewport` _returnvalue 0)
    (set `self.Cooldown` true)
    (`KismetSystemLibrary.Delay` 1.2)
    (set `self.Cooldown` false)
    (`Widget.RemoveFromParent` _returnvalue)))

(event `Use_Food1`
  (if (<= (`self.Food`) 0)
    (if (not (`self.Cooldown`))
      (bind _returnvalue (`|CreateWidget` "/Game/Custom/Widget/Dont_Have_Food.Dont_Have_Food_C"))
      (`UserWidget.AddToViewport` _returnvalue 0)
      (set `self.Cooldown` true)
      (`KismetSystemLibrary.Delay` 2.0)
      (set `self.Cooldown` false)
      (`Widget.RemoveFromParent` _returnvalue))
    (else
      (`self.Use_Food`)
      (if (`self.Poisoned_Character`)
        (set `self.Poisoned_Character` false)
        (bind _returnvalue_2 (`|CreateWidget` "/Game/Custom/Widget/Poisoned_Food.Poisoned_Food_C"))
        (`UserWidget.AddToViewport` _returnvalue_2 0)
        (`KismetSystemLibrary.Delay` 2.0)
        (`Widget.RemoveFromParent` _returnvalue_2)))))

(event `Use_Medicine1`
  (if (<= (`self.Medicines`) 0)
    (if (not (`self.Cooldown`))
      (bind _returnvalue (`|CreateWidget` "/Game/Custom/Widget/Dont_Have_Medkit.Dont_Have_Medkit_C"))
      (`UserWidget.AddToViewport` _returnvalue 0)
      (set `self.Cooldown` true)
      (`KismetSystemLibrary.Delay` 2.0)
      (set `self.Cooldown` false)
      (`Widget.RemoveFromParent` _returnvalue))
    (else
      (`self.Use_Medicine`))))

(event `Resting`
  (bind _returnvalue (`GameplayStatics.GetPlayerCameraManager` 0))
  (bind _returnvalue_2 (`GameplayStatics.GetPlayerPawn` 0))
  ;[1 1 1] Resting
  (if (`self.is_bed_near?`)
    (`Actor.DisableInput` _returnvalue_2 (`GameplayStatics.GetPlayerController` 0))
    (`self.Rest`)
    (set `self.Resting?` true)
    (`PlayerCameraManager.StartCameraFade` :`self` _returnvalue :`ToAlpha` 1.0 :`Duration` 2.5 :`bHoldWhenFinished` true)
    (`KismetSystemLibrary.Delay` 2.5)
    (`PlayerCameraManager.StartCameraFade` :`self` _returnvalue :`FromAlpha` 1.0 :`ToAlpha` 0.0 :`Duration` 2.5 :`bHoldWhenFinished` true)
    (`KismetSystemLibrary.Delay` 2.5)
    (`Actor.EnableInput` _returnvalue_2 (`GameplayStatics.GetPlayerController` 0))
    (set `self.Resting?` false)))

(fn `Add_Firematch`
  (set `self.Firematch` (+ (`self.Firematch`) 1)))

(fn `Add_Food`
  (bind _returnvalue (+ (`self.Food`) 1))
  (if (>= (`self.Food`) 1)
    (`self.Too_Much_Food`)
    (elif (> (`KismetMathLibrary.RandomInteger` 100) 95)
      (set `self.Food` _returnvalue)
      (set `self.Poisoned_Character` true)
      (else
        (set `self.Food` _returnvalue)))))

(fn `Add_Medicines`
  (bind _medicines (`self.Medicines`))
  (if (>= _medicines 1)
    (`self.Too_Much_Medicines`)
    (else
      (set `self.Medicines` (+ _medicines 1)))))

(fn `Create_UI`
  ;[1 1 1] Create UI
  (bind _returnvalue (`|CreateWidget` "/Game/Custom/Widget/UI_StatusBars.UI_StatusBars_C" (`GameplayStatics.GetPlayerController` 0)))
  (bind _output_get (set `self.UI` _returnvalue))
  (`UserWidget.AddToViewport` _output_get 0))

(fn `Health_degrowth_by_sanity_and_hunger`
  (bind _health_decrementation (`self.Health_decrementation`))
  (bind _is_hunger_zero_ (`self.Is_hunger_zero?`))
  (bind _returnvalue (- (`self.Health`) (`self.Health_decrementation`)))
  (bind _healthbar (`/Game/Custom/Widget/UI_StatusBars.HealthBar` (`self.UI`)))
  (bind _returnvalue_2 (<= _returnvalue 0.0))
  (if _returnvalue_2
    (set `self.Is_health_zero?` _returnvalue_2 :!label _label)
    (`ProgressBar.SetPercent` _healthbar _returnvalue)
    (`self.Death`)
    (elif (`self.Is_health_zero?`)
      (goto _label)
      (elif (`self.Is_sleep_zero?`)
        (if _is_hunger_zero_
          (set `self.Health_decrementation` (* _health_decrementation 2.0))
          (else
            (set `self.Health_decrementation` _health_decrementation :!label _label_2)))
        (bind _output_get (set `self.Health` _returnvalue))
        (`ProgressBar.SetPercent` _healthbar _output_get)
        (elif _is_hunger_zero_
          (goto _label_2))))))

(fn `Hunger_timer`
  (bind _returnvalue (- (`self.Hunger`) (`self.Hunger_decrementration`)))
  (bind _hungerbar (`/Game/Custom/Widget/UI_StatusBars.HungerBar` (`self.UI`)))
  (bind _returnvalue_2 (<= _returnvalue 0.0))
  (if _returnvalue_2
    (set `self.Is_hunger_zero?` _returnvalue_2 :!label _label)
    (bind _output_get (set `self.Hunger` 0.0))
    (`ProgressBar.SetPercent` _hungerbar _output_get)
    (else
      (set `self.Is_hunger_zero?` _returnvalue_2)
      (if (`self.Is_hunger_zero?`)
        (goto _label)
        (else
          (bind _output_get_2 (set `self.Hunger` _returnvalue))
          (`ProgressBar.SetPercent` _hungerbar _output_get_2))))))

(fn `Init_Parameters`
  (bind _ui (`self.UI`))
  (bind _ui_2 (`self.UI`))
  (bind _ui_3 (`self.UI`))
  ;[1 1 1] Init Sanity
  (bind _output_get (set `self.Sanity` 1.0))
  (`ProgressBar.SetPercent` (`/Game/Custom/Widget/UI_StatusBars.SanityBar` (`self.UI`)) _output_get)
  ;[1 1 1] Init Sleep
  (bind _output_get_2 (set `self.Sleep` 1.0))
  (`ProgressBar.SetPercent` (`/Game/Custom/Widget/UI_StatusBars.SleepBar` (`self.UI`)) _output_get_2)
  ;[1 1 1] Init Health
  (bind _output_get_3 (set `self.Health` 1.0))
  (`ProgressBar.SetPercent` (`/Game/Custom/Widget/UI_StatusBars.HealthBar` (`self.UI`)) _output_get_3)
  (set `self.Sanity_decrementation` (`self.Sanity_decrementation`))
  ;[1 1 1] Init Hunger
  (bind _output_get_4 (set `self.Hunger` 1.0))
  (`ProgressBar.SetPercent` (`/Game/Custom/Widget/UI_StatusBars.HungerBar` (`self.UI`)) _output_get_4)
  (set `self.Hunger_decrementration` (`self.Hunger_decrementration`))
  ;[1 1 1] Init Firematch Medicine and Food
  (bind _output_get_5 (set `self.Firematch` 1))
  (bind _output_get_6 (set `self.Medicines` 0))
  (bind _output_get_7 (set `self.Food` 0))
  (`EditableTextBox.SetHintText` (`/Game/Custom/Widget/UI_StatusBars.Firematch` _ui_2) (`KismetTextLibrary.Conv_ByteToText` (`KismetMathLibrary.Conv_IntToByte` _output_get_5)))
  (`EditableTextBox.SetHintText` (`/Game/Custom/Widget/UI_StatusBars.Medicine` _ui_2) (`KismetTextLibrary.Conv_ByteToText` (`KismetMathLibrary.Conv_IntToByte` _output_get_6)))
  (`EditableTextBox.SetHintText` (`/Game/Custom/Widget/UI_StatusBars.Food` _ui_2) (`KismetTextLibrary.Conv_ByteToText` (`KismetMathLibrary.Conv_IntToByte` _output_get_7)))
  ;[1 1 1] Init Time
  (set `self.Seconds` 0)
  (set `self.Minutes` 0)
  (set `self.Hours` 8)
  (set `self.Days` 1)
  (`EditableTextBox.SetHintText` (`/Game/Custom/Widget/UI_StatusBars.Days` _ui_3) (`KismetTextLibrary.Conv_ByteToText` 1))
  (`EditableTextBox.SetHintText` (`/Game/Custom/Widget/UI_StatusBars.Minutes` _ui_3) (`KismetTextLibrary.Conv_ByteToText` 0))
  (`EditableTextBox.SetHintText` (`/Game/Custom/Widget/UI_StatusBars.Hours` _ui_3) (`KismetTextLibrary.Conv_ByteToText` 8))
  ;[1 1 1] Init Icons visibility
  (`Widget.SetVisibility` (`/Game/Custom/Widget/UI_StatusBars.Sanity100-75` _ui) "Hidden")
  (`Widget.SetVisibility` (`/Game/Custom/Widget/UI_StatusBars.Sanity75-30` _ui) "Hidden")
  (`Widget.SetVisibility` (`/Game/Custom/Widget/UI_StatusBars.Sanity30-0` _ui) "Hidden")
  (`Widget.SetVisibility` (`/Game/Custom/Widget/UI_StatusBars.Sanity<0` _ui) "Hidden"))

(fn `Rest`
  (bind _sleep (`self.Sleep`))
  (bind _ui (`self.UI`))
  (bind _returnvalue (+ (`self.Days`) 1))
  (set `self.Seconds` 0)
  (bind _output_get (set `self.Hours` 8))
  (set `self.Days` _returnvalue)
  (`EditableTextBox.SetHintText` (`/Game/Custom/Widget/UI_StatusBars.Hours` _ui) (`KismetTextLibrary.Conv_ByteToText` _output_get))
  (`EditableTextBox.SetHintText` (`/Game/Custom/Widget/UI_StatusBars.Days` _ui) (`KismetTextLibrary.Conv_IntToText` _returnvalue))
  (if (< _sleep 0.3)
    (set `self.Sleep` 0.75)
    (else
      (set `self.Sleep` 1.0)))
  (`ProgressBar.SetPercent` (`/Game/Custom/Widget/UI_StatusBars.SleepBar` _ui) _sleep))

(fn `Sanity_timer`
  (bind _sanity (`self.Sanity`))
  (bind _ui (`self.UI`))
  (bind _returnvalue (- _sanity (`self.Sanity_decrementation`)))
  (bind _sanity100_75 (`/Game/Custom/Widget/UI_StatusBars.Sanity100-75` _ui))
  (bind _sanity75_30 (`/Game/Custom/Widget/UI_StatusBars.Sanity75-30` _ui))
  (bind _sanity30_0 (`/Game/Custom/Widget/UI_StatusBars.Sanity30-0` _ui))
  (bind _sanity_0 (`/Game/Custom/Widget/UI_StatusBars.Sanity<0` _ui))
  (bind _returnvalue_2 (<= _returnvalue 1e-05))
  (if (`self.Resting?`)
    _
    (elif (not (`self.Is_in_light?`))
      (if (>= _sanity 1.0)
        (set `self.Sanity` 1.0))
      (if _returnvalue_2
        (set `self.Is_sanity_zero?` _returnvalue_2 :!label _label)
        (`Widget.SetVisibility` _sanity100_75 "Hidden" :!label _label_2)
        (`Widget.SetVisibility` _sanity75_30 "Hidden")
        (`Widget.SetVisibility` _sanity30_0 "Hidden")
        (`Widget.SetVisibility` _sanity_0 "Visible")
        (elif (`self.Is_sanity_zero?`)
          (goto _label)
          (else
            (bind _output_get (set `self.Sanity` _returnvalue))
            (`ProgressBar.SetPercent` (`/Game/Custom/Widget/UI_StatusBars.SanityBar` (`self.UI`)) _output_get)
            (if (> _output_get 0.75)
              ;[1 1 1] Sanity Rannge Flags Settings
              (set `self.Low_Sanity` false)
              (set `self.Medium_Sanity` false)
              (set `self.Full_Sanity` true)
              (`Widget.SetVisibility` _sanity100_75 "Visible")
              (`Widget.SetVisibility` _sanity75_30 "Hidden")
              (`Widget.SetVisibility` _sanity30_0 "Hidden")
              (`Widget.SetVisibility` _sanity_0 "Hidden")
              (elif (> _output_get 0.3)
                (set `self.Low_Sanity` false)
                (set `self.Medium_Sanity` true)
                (set `self.Full_Sanity` false)
                (`Widget.SetVisibility` _sanity100_75 "Hidden")
                (`Widget.SetVisibility` _sanity75_30 "Visible")
                (`Widget.SetVisibility` _sanity30_0 "Hidden")
                (`Widget.SetVisibility` _sanity_0 "Hidden")
                (else
                  (set `self.Low_Sanity` true)
                  (set `self.Medium_Sanity` false)
                  (set `self.Full_Sanity` false)
                  (if (> _output_get 2e-05)
                    (`Widget.SetVisibility` _sanity100_75 "Hidden")
                    (`Widget.SetVisibility` _sanity75_30 "Hidden")
                    (`Widget.SetVisibility` _sanity30_0 "Visible")
                    (`Widget.SetVisibility` _sanity_0 "Hidden")
                    (else
                      (goto _label_2))))))))))))

(fn `Sleep_Timer`
  (bind _returnvalue (- (`self.Sleep`) (`self.Sleep_Decrementation`)))
  (bind _sleepbar (`/Game/Custom/Widget/UI_StatusBars.SleepBar` (`self.UI`)))
  (bind _returnvalue_2 (<= _returnvalue 0.0))
  (if _returnvalue_2
    (set `self.Is_sleep_zero?` _returnvalue_2 :!label _label)
    (set `self.Sleep` 0.0)
    (`ProgressBar.SetPercent` _sleepbar 0.0)
    (else
      (set `self.Is_sleep_zero?` _returnvalue_2)
      (if (`self.Is_sleep_zero?`)
        (goto _label)
        (else
          (bind _output_get (set `self.Sleep` _returnvalue))
          (`ProgressBar.SetPercent` _sleepbar _output_get))))))

(fn `Time`
  (bind _ui (`self.UI`))
  (bind _ui_2 (`self.UI`))
  (bind _output_get (set `self.Seconds` (+ (`self.Seconds`) 1)))
  (if (>= _output_get 1)
    (set `self.Seconds` 0)
    (bind _output_get_2 (set `self.Minutes` (+ (`self.Minutes`) 1)))
    (if (>= _output_get_2 60)
      (bind _output_get_3 (set `self.Minutes` 0))
      (bind _output_get_4 (set `self.Hours` (+ (`self.Hours`) 1)))
      (if (>= _output_get_4 24)
        (set `self.Hours` 0)
        (bind _output_get_5 (set `self.Days` (+ (`self.Days`) 1)))
        (`EditableTextBox.SetHintText` (`/Game/Custom/Widget/UI_StatusBars.Days` _ui_2) (`KismetTextLibrary.Conv_IntToText` _output_get_5))
        (`EditableTextBox.SetHintText` (`/Game/Custom/Widget/UI_StatusBars.Minutes` _ui_2) (`KismetTextLibrary.Conv_ByteToText` 0))
        (`EditableTextBox.SetHintText` (`/Game/Custom/Widget/UI_StatusBars.Hours` _ui_2) (`KismetTextLibrary.Conv_ByteToText` 0))
        (`/Engine/EditorBlueprintResources/StandardMacros.DoOnce` false :!via `Reset`)
        (else
          (`EditableTextBox.SetHintText` (`/Game/Custom/Widget/UI_StatusBars.Minutes` _ui) (`KismetTextLibrary.Conv_ByteToText` _output_get_3))
          (`EditableTextBox.SetHintText` (`/Game/Custom/Widget/UI_StatusBars.Hours` _ui) (`KismetTextLibrary.Conv_ByteToText` _output_get_4))))
      (else
        (`EditableTextBox.SetHintText` (`/Game/Custom/Widget/UI_StatusBars.Minutes` (`self.UI`)) (`KismetTextLibrary.Conv_ByteToText` _output_get_2))))))

(fn `Use_Food`
  (bind _food (`self.Food`))
  (bind _ui (`self.UI`))
  (bind _ui_2 (`self.UI`))
  (bind _food_2 (`self.Food`))
  (if (`self.Poisoned_Character`)
    (if (> _food 0)
      (bind _output_get (set `self.Food` (- _food 1)))
      (bind _output_get_2 (set `self.Hunger` (+ (`self.Hunger`) 0.25)))
      (bind _output_get_3 (set `self.Health` (- (`self.Health`) 0.2)))
      (`ProgressBar.SetPercent` (`/Game/Custom/Widget/UI_StatusBars.HealthBar` _ui) _output_get_3)
      (`ProgressBar.SetPercent` (`/Game/Custom/Widget/UI_StatusBars.HungerBar` _ui) _output_get_2)
      (`EditableTextBox.SetHintText` (`/Game/Custom/Widget/UI_StatusBars.Food` _ui) (`KismetTextLibrary.Conv_IntToText` _output_get)))
    (elif (> _food_2 0)
      (bind _output_get_4 (set `self.Food` (- _food_2 1)))
      (bind _output_get_5 (set `self.Hunger` (+ (`self.Hunger`) 0.25)))
      (`ProgressBar.SetPercent` (`/Game/Custom/Widget/UI_StatusBars.HungerBar` _ui_2) _output_get_5)
      (`EditableTextBox.SetHintText` (`/Game/Custom/Widget/UI_StatusBars.Food` _ui_2) (`KismetTextLibrary.Conv_IntToText` _output_get_4)))))

(fn `Use_Medicine`
  (bind _medicines (`self.Medicines`))
  (bind _ui (`self.UI`))
  (if (> _medicines 0)
    (bind _output_get (set `self.Medicines` (- _medicines 1)))
    (bind _output_get_2 (set `self.Health` (+ (`self.Health`) 0.2)))
    (`ProgressBar.SetPercent` (`/Game/Custom/Widget/UI_StatusBars.HealthBar` _ui) _output_get_2)
    (`EditableTextBox.SetHintText` (`/Game/Custom/Widget/UI_StatusBars.Medicine` _ui) (`KismetTextLibrary.Conv_IntToText` _output_get))))